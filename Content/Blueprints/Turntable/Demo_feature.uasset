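; Idle attract-mode controller for the vehicle turntable showroom, starting a looping demo sequence after a period without input.
; Key or axis input stops the demo and restarts the idle timer via a retriggerable delay.
; Tick watches Phase for changes, dispatching steps that toggle UI and controls, cycle vehicles, and force materials or environments.
; DemoSetup caches turntable, pawn, vehicle and widget references, which a validation macro re-acquires when invalid.
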(event Custom|stop_demo
  (Utilities|FlowControl|DoOnce true
    (:Completed
      (Sequencer|Player|Stop (Variables|/Script/LevelSequence.LevelSequenceActor|GetSequencePlayer (Variables|Default|Getdemo%20sequence)) :!class /Script/MovieScene.MovieSceneSequencePlayer))))

(event Custom|start_demo
  (bind _demo_sequence (Variables|Default|Getdemo%20sequence))
  (bind _sequenceplayer (Variables|/Script/LevelSequence.LevelSequenceActor|GetSequencePlayer _demo_sequence))
  (Class|MovieSceneSequencePlayer|PlayLooping _sequenceplayer -1)
  (Utilities|FlowControl|DoOnce true) ; enters at Reset
)

(event Custom|next%20phase
  (bind _turntable_controlls (Variables|Default|Getturntable_controlls))
  (bind _turntable (Variables|Default|Getturntable))
  (bind _pawn (Variables|Default|Getpawn))
  (bind _vehicle (Variables|Default|Getvehicle))
  (bind _turntable_2 (Variables|Default|Getturntable))
  (bind _turntable_3 (Variables|Default|Getturntable))
  (bind _vehicle_2 (Variables|/Game/Blueprints/Turntable/Turntable_system_controler.Turntable_system_controler_C|Getvehicle _turntable))
  (switch int (Variables|Default|GetPhase)
    (:0
      (Default|RemoveControlls _pawn)
      (Default|HUDToggle _pawn)
      (Utilities|DemoObjectValidation _turntable_controlls
        (:Is%20Valid
          (Default|ActivateMenu _turntable_controlls))))
    (:1
      (Utilities|DemoObjectValidation _turntable
        (:Is%20Valid
          (bind _result (Math|Integer|IncrementInt (Variables|Default|Getvehicle%20num))
            (:%20%20
              (if (>= _result (Utilities|Array|LastIndex _vehicle_2))
                (Variables|Default|Setvehicle%20num 0))
              (Default|SpawnVehicle _turntable (Utilities|Array|Get(acopy) _vehicle_2 (Variables|Default|Getvehicle%20num)))
              (Variables|Default|Setis%20vid (Utilities|Enum|Equal(Enum) (.Name (Utilities|GetClassDefaults (Utilities|Array|Get(acopy) _vehicle_2 (Variables|Default|Getvehicle%20num)))) "ARCHITECHTURE"))
              (if (Variables|Default|Getis%20vid)
                (Sequencer|Player|Pause (Variables|/Script/LevelSequence.LevelSequenceActor|GetSequencePlayer (Variables|Default|Getdemo%20sequence)))
                (else
                  (Utilities|FlowControl|Delay 2.0))))))))
    (:2
      (Utilities|DemoObjectValidation _vehicle
        (:Is%20Valid
          (Default|ForceMatChange _vehicle 2)
          (Utilities|DemoObjectValidation _turntable_2
            (:Is%20Valid
              (Default|ForceShowroomEnviron _turntable_2))))))
    (:3
      (Utilities|DemoObjectValidation _turntable_3
        (:Is%20Valid
          (Default|ForceForestEnvironment _turntable_3))))))

(event EventBeginPlay
  (Class|KismetMathLibrary|SeedRandomStream (Variables|Default|Getrandom))
  (Utilities|FlowControl|Delay 3.0)
  (bind _valid (CallFunction|DemoSetup))
  (if _valid
    (Utilities|FlowControl|RetriggerableDelay (Variables|Default|GetIdle%20time))
    (CallFunction|StartDemo)
    (else
      (Development|PrintString "VALIDATION ERROR:1" true true "(R=1.000000,G=0.000000,B=0.000000,A=1.000000)" 1e+01))))

(event EventTick
  (params (DeltaSeconds :type Float%20%28single-precision%29))
  (bind _phase (Variables|Default|GetPhase))
  (if (!= (+ (Math|Float|Absolute(Float) (Class|Actor|GetInputAxisKeyValue)) (Math|Float|Absolute(Float) (Class|Actor|GetInputAxisKeyValue)) (Math|Float|Absolute(Float) (Class|Actor|GetInputAxisKeyValue))) 0.0)
    (CallFunction|StopDemo)
    (Utilities|FlowControl|RetriggerableDelay (Variables|Default|GetIdle%20time))
    (CallFunction|StartDemo)
    (elif (not (== _phase (Variables|Default|Getold%20phase)))
      (Variables|Default|Setold%20phase _phase)
      (CallFunction|NextPhase))))

(event Input|KeyboardEvents|AnyKey
  (params (Key :type Key%20Structure))
  (:Pressed
    (CallFunction|StopDemo)
    (Utilities|FlowControl|RetriggerableDelay (Variables|Default|GetIdle%20time))
    (CallFunction|StartDemo)))

(fn ConstructionScript)

(fn DemoSetup
  (bind _foundwidgets (Widget|GetAllWidgetsOfClass "/Game/Blueprints/Turntable/Turntable_controls_alt.Turntable_controls_alt_C" false))
  (Variables|Default|Setturntable_controlls (Utilities|Array|Get(acopy) _foundwidgets (Utilities|Array|LastIndex _foundwidgets)))
  (bind _outactors (Actor|GetAllActorsOfClass "/Game/Blueprints/Turntable/Vehicle_Viewer.Vehicle_Viewer_C"))
  (Variables|Default|Setvehicle (Utilities|Array|Get(acopy) _outactors (Utilities|Array|LastIndex _outactors)))
  (bind _outactors_2 (Actor|GetAllActorsOfClass "/Game/Blueprints/Turntable/Turntable_system_controler.Turntable_system_controler_C"))
  (Variables|Default|Setturntable (Utilities|Array|Get(acopy) _outactors_2 (Utilities|Array|LastIndex _outactors_2)))
  (bind _asturntable_pawn (Utilities|Casting|CastToTurntable_Pawn (Game|Player|GetPlayerPawn 0)))
  (Variables|Default|Setpawn _asturntable_pawn)
  (LocalVariables|Setvalidation true)
  (bind (_array_element _array_index) (Utilities|Array|ForEachLoopwithBreak (Utilities|Array|MakeArray (Variables|Default|Getturntable_controlls) (Variables|Default|Getvehicle) (Variables|Default|Getturntable) (Variables|Default|Getpawn) (Variables|Default|Getdemo%20sequence)) :!label _label)
    (:LoopBody
      (Utilities|IsValid _array_element
        (:Is%20Not%20Valid
          (Development|PrintString (Utilities|String|ToString(Integer) _array_index) true true "(R=1.000000,G=0.021000,B=0.000000,A=1.000000)" 1e+01)
          (LocalVariables|Setvalidation false)
          (goto _label Break))))
    (:Completed
      (return (LocalVariables|Getvalidation)))))