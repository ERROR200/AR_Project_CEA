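; Turntable controller actor that spawns display vehicles and switches the streamed environment around them.
; spawn_vehicle kills the current vehicle, then spawns the requested class if it is in the Vehicle list.
; Environment events stream the showroom (loaded at BeginPlay) or landscape test level, unloading the other and toggling the mesh's visibility; a looping MultiGate alternates them.
; settime stores a time value; basic and water environment logic is left unconnected.
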(event Custom|spawn_%20vehicle
  (params (ItemToFind :type Vehicle%20Viewer%20Class%20Reference%20%28by%20ref%29))
  (bind _vehicle (Variables|Default|Getvehicle))
  (bind _returnvalue (Utilities|Array|FindItem _vehicle ItemToFind))
  (Utilities|IsValid (Variables|Default|Getcurrent%20vehicle)
    (:Is%20Valid
      (Default|Kill (Variables|Default|Getcurrent%20vehicle)))
    (:Is%20Not%20Valid
      _))
  (if (== _returnvalue -1)
    (Development|PrintString "ERROR: Vehicle not found")
    (else
      (bind _returnvalue_2 (Game|SpawnActorfromClass (Utilities|Array|Get(acopy) _vehicle _returnvalue) (Math|Transform|MakeTransform "0, 0,2.500000" "0, 0, 0" "1,1,1") "AlwaysSpawn" 0 0))
      (Variables|Default|Setcurrent%20vehicle _returnvalue_2))))

(event Custom|toggle%20environment
  (bind _staticmeshcomponent (Variables|Debug|GetStaticMeshComponent))
  (Utilities|FlowControl|MultiGate false true 1
    (:Out%200
      (Variables|Default|SetEnviro_index 1)
      (Development|SetHiddeninGame _staticmeshcomponent false false)
      (Game|LoadStreamLevel(byName) "TurnTable_Showroom" true)
      (Game|UnloadStreamLevel(byName) "TurnTable_landscapeTest"))
    (:Out%201
      (Variables|Default|SetEnviro_index 2)
      (Development|SetHiddeninGame _staticmeshcomponent true false)
      (Game|LoadStreamLevel(byName) "TurnTable_landscapeTest" true)
      (Game|UnloadStreamLevel(byName) "TurnTable_Showroom"))))

(event Custom|force%20forest%20environment
  (Variables|Default|SetEnviro_index 2)
  (Development|SetHiddeninGame (Variables|Debug|GetStaticMeshComponent) true false)
  (Game|LoadStreamLevel(byName) "TurnTable_landscapeTest" true)
  (Game|UnloadStreamLevel(byName) "TurnTable_Showroom"))

(event Custom|force_basic_environ)

(event Custom|force%20showroom%20environ
  (Variables|Default|SetEnviro_index 1)
  (Development|SetHiddeninGame (Variables|Debug|GetStaticMeshComponent) false false)
  (Game|LoadStreamLevel(byName) "TurnTable_Showroom" true)
  (Game|UnloadStreamLevel(byName) "TurnTable_landscapeTest"))

(event Custom|set%20time
  (params (time :type Float%20%28single-precision%29))
  (Variables|Default|Settime time))

(event Collision|EventActorBeginOverlap
  (params (OtherActor :type Actor%20Object%20Reference)))

(event EventTick
  (params (DeltaSeconds :type Float%20%28single-precision%29)))

(event EventBeginPlay
  (Development|SetHiddeninGame (Variables|Debug|GetStaticMeshComponent) false false)
  (Game|LoadStreamLevel(byName) "TurnTable_Showroom" true)
  (Game|UnloadStreamLevel(byName) "TurnTable_landscapeTest"))

(fn ConstructionScript)