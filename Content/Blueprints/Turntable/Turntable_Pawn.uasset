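; Player pawn for a vehicle turntable viewer, with a spring-arm camera, controls overlay and idle prompts.
; Input restarts retriggerable delays: a Tick-fed gate resumes auto-spin after a short pause, and a longer wait shows the idle screen.
; Wheel zoom, faster with Shift, syncs the widget slider and Vehicle_Viewer.
; Right-click toggles the overlay, Escape quits, and a looping timer watches camera rotation to dismiss the drag hint.
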(event Custom|Set_zoom_limit
  (params (iso%20mode :type Boolean))
  (bind _widget (Variables|Default|GetWidget))
  ;[1 1 1] Zoom Handle
  (if iso%20mode
    (Variables|Default|Setmin_zoom 2e+02)
    (else
      (Variables|Default|Setmin_zoom 5e+02)))
  (Variables|/Script/Engine.SpringArmComponent|SetTargetArmLength (Variables|Default|GetSpringArm) (Variables|Default|GetSpring%20arm%20length))
  (Utilities|IsValid _widget
    (:Is%20Valid
      (Default|SetZoomSlider _widget (Math|Float|MapRangeClamped (Variables|Default|GetSpring%20arm%20length) 1.3e+03 (Variables|Default|Getmin_zoom) 0.0 1.0))
      (bind _outactors (Actor|GetAllActorsOfClass "/Game/Blueprints/Turntable/Vehicle_Viewer.Vehicle_Viewer_C"))
      (Utilities|IsValid (Utilities|Array|Get(acopy) _outactors)
        (:Is%20Valid
          (Default|ChangeZoom (Utilities|Array|Get(acopy) _outactors) (Math|Float|MapRangeClamped (Variables|Default|GetSpring%20arm%20length) (Variables|Default|Getmin_zoom) 1.3e+03 0.0 1.0)))))))

(event Custom|show%20hud
  (bind _returnvalue (Viewport|GetViewportSize))
  (bind _returnvalue_2 (Game|GetPlayerController 0))
  (if (not (Variables|Default|Getoverlay_visable))
    (bind _foundwidgets (Widget|GetAllWidgetsOfClass "/Game/Blueprints/Turntable/User_Interface/TurnTable_Anim_UI.TurnTable_Anim_UI_C" false))
    (Variables|Default|Setanim_widget (Utilities|Array|Get(acopy) _foundwidgets (Utilities|Array|LastIndex _foundwidgets)))
    ;[1 1 1] Hud Toggle
    (Variables|Default|Setoverlay_visable true)
    (UserInterface|Viewport|AddtoViewport (Variables|Default|GetWidget) 0)
    (Utilities|IsValid (Variables|Default|Getanim_widget)
      (:Is%20Valid
        (Default|Hide (Variables|Default|Getanim_widget) true))
      (:Is%20Not%20Valid
        _))
    (Variables|/Script/Engine.PlayerController|SetbShowMouseCursor _returnvalue_2 true)
    (Input|SetInputModeGameandUI _returnvalue_2 0 "DoNotLock" false)
    (Class|PlayerController|SetMouseLocation _returnvalue_2 (/ (Math|Float|Truncate (.x _returnvalue)) 2) (/ (Math|Float|Truncate (.y _returnvalue)) 2))))

(event Custom|idle
  (Variables|Default|Setis%20idle true)
  (bind _returnvalue (UserInterface|CreateWidget "/Game/Blueprints/Turntable/User_Interface/IDLE_MESSAGE.IDLE_MESSAGE_C"))
  (UserInterface|Viewport|AddtoViewport _returnvalue 100)
  (Variables|Default|Setilde_ui _returnvalue)
  (CallFunction|ShowHud)
  (Default|ForceMenu (Variables|Default|GetWidget))
  (CallFunction|StopDragMessege))

(event Custom|hide%20idle
  (Variables|Default|Setis%20idle false)
  (Utilities|IsValid (stale Custom|idle _returnvalue)
    (:Is%20Valid
      (Widget|RemovefromParent (stale Custom|idle _returnvalue)))))

(event Custom|update_spin_speed
  (params (spin_speed :type Float%20%28single-precision%29))
  ;[1 1 1] Spin Automation
  (Variables|Default|Setspin_speed spin_speed) ; Change Spin Speed
)

(event Custom|set%20zoom%20w/%20bar
  (params (TargetArmLength :type Float%20%28single-precision%29))
  (bind _output_get (Variables|Default|SetSpring%20arm%20length (Math|Float|Lerp 1.3e+03 (Variables|Default|Getmin_zoom) TargetArmLength)))
  (Variables|/Script/Engine.SpringArmComponent|SetTargetArmLength (Variables|Default|GetSpringArm) _output_get)
  ;[1 1 1] Zoom Handle
  (bind _outactors (Actor|GetAllActorsOfClass "/Game/Blueprints/Turntable/Vehicle_Viewer.Vehicle_Viewer_C"))
  (Utilities|IsValid (Utilities|Array|Get(acopy) _outactors)
    (:Is%20Valid
      (Default|ChangeZoom (Utilities|Array|Get(acopy) _outactors) (Math|Float|MapRangeClamped (Variables|Default|GetSpring%20arm%20length) (Variables|Default|Getmin_zoom) 1.3e+03 0.0 1.0)))))

(event Custom|camera%20movement%20check
  (bind _returnvalue (Utilities|Time|SetTimerbyEvent (delegate Custom|camera%20movement%20check) 0.05 true))
  (if (Utilities|Enum|NotEqual(Enum) (Variables|Default|Getidle%20camera%20rotation) (Class|SpringArmComponent|GetTargetRotation (Variables|Default|GetSpringArm)) 1e+01)
    (Utilities|Time|ClearandInvalidateTimerbyHandle _returnvalue)
    (Utilities|IsValid (stale Custom|drag%20screen%20messege _returnvalue)
      (:Is%20Valid
        (Widget|RemovefromParent (stale Custom|drag%20screen%20messege _returnvalue))))))

(event Custom|idle%20wake
  (bind _ilde_ui (Variables|Default|Getilde_ui))
  ;[1 1 1] Spin Automation
  (Utilities|FlowControl|Sequence
    (:then_0
      (Utilities|FlowControl|Gate false) ; enters at Close
    )
    (:then_1
      (Utilities|FlowControl|RetriggerableDelay 3.0) ; Auto Rotate Delay
      (if (not (== (Variables|Default|Getspin_speed) 0.0)) ; Is Spin Paused
        (Utilities|FlowControl|Gate false) ; enters at Open
      ))
    (:then_2
      (Utilities|FlowControl|RetriggerableDelay 3e+01) ; idle delay
      (CallFunction|Idle)
      (Variables|Default|Setwas%20idle true))
    (:then_3
      (if (Variables|Default|Getis%20idle)
        (Variables|Default|Setis%20idle false)
        (Utilities|IsValid _ilde_ui
          (:Is%20Valid
            (Widget|RemovefromParent _ilde_ui)))))))

(event Custom|stop%20drag%20messege
  (Utilities|Time|ClearandInvalidateTimerbyHandle (stale Custom|camera%20movement%20check _returnvalue))
  (Utilities|IsValid (stale Custom|drag%20screen%20messege _returnvalue)
    (:Is%20Valid
      (Widget|RemovefromParent (stale Custom|drag%20screen%20messege _returnvalue)))))

(event Custom|drag%20screen%20messege
  (if (Variables|Default|Getwas%20idle)
    (Variables|Default|Setwas%20idle false)
    (Variables|Default|Setidle%20camera%20rotation (Class|SpringArmComponent|GetTargetRotation (Variables|Default|GetSpringArm)))
    (CallFunction|CameraMovementCheck)
    (bind _returnvalue (UserInterface|CreateWidget "/Game/Blueprints/Turntable/User_Interface/dragscreen_MESSAGE.dragscreen_MESSAGE_C"))
    (UserInterface|Viewport|AddtoViewport _returnvalue 100)))

(event Custom|HUD%20Toggle
  (bind _returnvalue (Viewport|GetViewportSize))
  (bind _returnvalue_2 (Game|GetPlayerController 0))
  (bind _widget (Variables|Default|GetWidget))
  (bind _foundwidgets (Widget|GetAllWidgetsOfClass "/Game/Blueprints/Turntable/User_Interface/TurnTable_Anim_UI.TurnTable_Anim_UI_C" false))
  (Variables|Default|Setanim_widget (Utilities|Array|Get(acopy) _foundwidgets (Utilities|Array|LastIndex _foundwidgets)))
  ;[1 1 1] Hud Toggle
  (if (Variables|Default|Getoverlay_visable)
    (Variables|Default|Setoverlay_visable false)
    (Widget|RemovefromParent _widget)
    (Utilities|IsValid (Variables|Default|Getanim_widget)
      (:Is%20Valid
        (Default|Hide (Variables|Default|Getanim_widget) false))
      (:Is%20Not%20Valid
        _))
    (Variables|/Script/Engine.PlayerController|SetbShowMouseCursor _returnvalue_2 false)
    (Input|SetInputModeGameOnly _returnvalue_2)
    (Class|WidgetBlueprintLibrary|SetFocustoGameViewport)
    (else
      (Variables|Default|Setoverlay_visable true)
      (UserInterface|Viewport|AddtoViewport _widget 0)
      (Utilities|IsValid (Variables|Default|Getanim_widget)
        (:Is%20Valid
          (Default|Hide (Variables|Default|Getanim_widget) true))
        (:Is%20Not%20Valid
          _))
      (Variables|/Script/Engine.PlayerController|SetbShowMouseCursor _returnvalue_2 true)
      (Input|SetInputModeGameandUI _returnvalue_2 0 "DoNotLock" false)
      (Class|PlayerController|SetMouseLocation _returnvalue_2 (/ (Math|Float|Truncate (.x _returnvalue)) 2) (/ (Math|Float|Truncate (.y _returnvalue)) 2)))))

(event Custom|remove%20controlls
  (bind _returnvalue (Game|GetPlayerController 0))
  ;[1 1 1] Hud Toggle
  (Variables|Default|Setoverlay_visable false)
  (bind _foundwidgets (Widget|GetAllWidgetsOfClass "/Game/Blueprints/Turntable/User_Interface/TurnTable_Anim_UI.TurnTable_Anim_UI_C" false))
  (Variables|Default|Setanim_widget (Utilities|Array|Get(acopy) _foundwidgets (Utilities|Array|LastIndex _foundwidgets)))
  (Widget|RemovefromParent (Variables|Default|GetWidget))
  (Utilities|IsValid (Variables|Default|Getanim_widget)
    (:Is%20Valid
      (Default|Hide (Variables|Default|Getanim_widget) false))
    (:Is%20Not%20Valid
      _))
  (Variables|/Script/Engine.PlayerController|SetbShowMouseCursor _returnvalue false)
  (Input|SetInputModeGameOnly _returnvalue)
  (Class|WidgetBlueprintLibrary|SetFocustoGameViewport))

(event EventBeginPlay
  (bind _returnvalue (Viewport|GetViewportSize))
  (bind _returnvalue_2 (Game|GetPlayerController 0))
  (bind _anim_widget (Variables|Default|Getanim_widget))
  ;[1 1 1] Initial Setup
  (Variables|/Script/Engine.SpringArmComponent|SetTargetArmLength (Variables|Default|GetSpringArm) (Variables|Default|GetSpring%20arm%20length))
  (bind _returnvalue_3 (UserInterface|CreateWidget "/Game/Blueprints/Turntable/User_Interface/Turntable_controls_alt.Turntable_controls_alt_C"))
  (Variables|Default|SetWidget _returnvalue_3)
  (Default|BeginSystem _returnvalue_3)
  (Development|ExecuteConsoleCommand "r.PostProcessAAQuality 5" 0)
  (Utilities|FlowControl|Delay 0.5)
  (Variables|/Script/Engine.SpringArmComponent|SetbUsePawnControlRotation (Variables|Default|GetSpringArm) true)
  (CallFunction|Idle)
  ;[1 1 1] Hud Toggle
  (UserInterface|Viewport|AddtoViewport (Variables|Default|GetWidget) 0)
  (Utilities|IsValid _anim_widget
    (:Is%20Valid
      (Default|Hide _anim_widget true))
    (:Is%20Not%20Valid
      _))
  (Variables|/Script/Engine.PlayerController|SetbShowMouseCursor _returnvalue_2 true)
  (Input|SetInputModeGameandUI _returnvalue_2 0 "DoNotLock" false)
  (Class|PlayerController|SetMouseLocation _returnvalue_2 (/ (Math|Float|Truncate (.x _returnvalue)) 2) (/ (Math|Float|Truncate (.y _returnvalue)) 2)))

(event EventTick
  (params (DeltaSeconds :type Float%20%28single-precision%29))
  (bind _ilde_ui (Variables|Default|Getilde_ui))
  ;[1 1 1] Spin Automation
  (if (!= (+ (Math|Float|Absolute(Float) (Class|Actor|GetInputAxisKeyValue)) (Math|Float|Absolute(Float) (Class|Actor|GetInputAxisKeyValue)) (Math|Float|Absolute(Float) (Class|Actor|GetInputAxisKeyValue))) 0.0) ; Is Camera Not Moving?
    (Utilities|FlowControl|Sequence
      (:then_0
        (goto _label Close))
      (:then_1
        (Utilities|FlowControl|RetriggerableDelay 3.0) ; Auto Rotate Delay
        (if (not (== (Variables|Default|Getspin_speed) 0.0)) ; Is Spin Paused
          (goto _label Open)))
      (:then_2
        (Utilities|FlowControl|RetriggerableDelay 3e+01) ; idle delay
        (CallFunction|Idle)
        (Variables|Default|Setwas%20idle true))
      (:then_3
        (if (Variables|Default|Getis%20idle)
          (Variables|Default|Setis%20idle false)
          (Utilities|IsValid _ilde_ui
            (:Is%20Valid
              (Widget|RemovefromParent _ilde_ui))))))
    (else
      (Utilities|FlowControl|Gate false :!label _label
        (:Exit
          (Pawn|Input|AddControllerYawInput (Variables|Default|Getspin_speed)) ; Spin
        )))))

(event Input|KeyboardEvents|Escape
  (params (Key :type Key%20Structure))
  ;[1 1 1] Quit Game
  (:Pressed
    (Game|QuitGame 0 "Quit")))

(event Input|MouseEvents|MouseWheelDown
  (params (Key :type Key%20Structure))
  (bind _widget (Variables|Default|GetWidget))
  (bind _min_zoom (Variables|Default|Getmin_zoom))
  ;[1 1 1] Zoom Handle
  (:Pressed
    (Utilities|ModifyerCheck
      (:false
        (Variables|Default|SetSpring%20arm%20length (Math|Float|Clamp(Float) (+ (Variables|Default|GetSpring%20arm%20length) 5e+01) _min_zoom 1.3e+03)))
      (:true
        (Variables|Default|SetSpring%20arm%20length (Math|Float|Clamp(Float) (+ (Variables|Default|GetSpring%20arm%20length) 2e+02) _min_zoom 1.3e+03))))
    (Variables|/Script/Engine.SpringArmComponent|SetTargetArmLength (Variables|Default|GetSpringArm) (Variables|Default|GetSpring%20arm%20length))
    (Utilities|IsValid _widget
      (:Is%20Valid
        (Default|SetZoomSlider _widget (Math|Float|MapRangeClamped (Variables|Default|GetSpring%20arm%20length) 1.3e+03 (Variables|Default|Getmin_zoom) 0.0 1.0))
        (bind _outactors (Actor|GetAllActorsOfClass "/Game/Blueprints/Turntable/Vehicle_Viewer.Vehicle_Viewer_C"))
        (Utilities|IsValid (Utilities|Array|Get(acopy) _outactors)
          (:Is%20Valid
            (Default|ChangeZoom (Utilities|Array|Get(acopy) _outactors) (Math|Float|MapRangeClamped (Variables|Default|GetSpring%20arm%20length) (Variables|Default|Getmin_zoom) 1.3e+03 0.0 1.0))))))))

(event Input|KeyboardEvents|AnyKey
  (params (Key :type Key%20Structure))
  (bind _ilde_ui (Variables|Default|Getilde_ui))
  ;[1 1 1] Spin Automation
  (:Pressed
    (Utilities|FlowControl|Sequence
      (:then_0
        (Utilities|FlowControl|Gate false) ; enters at Close
      )
      (:then_1
        (Utilities|FlowControl|RetriggerableDelay 3.0) ; Auto Rotate Delay
        (if (not (== (Variables|Default|Getspin_speed) 0.0)) ; Is Spin Paused
          (Utilities|FlowControl|Gate false) ; enters at Open
        ))
      (:then_2
        (Utilities|FlowControl|RetriggerableDelay 3e+01) ; idle delay
        (CallFunction|Idle)
        (Variables|Default|Setwas%20idle true))
      (:then_3
        (if (Variables|Default|Getis%20idle)
          (Variables|Default|Setis%20idle false)
          (Utilities|IsValid _ilde_ui
            (:Is%20Valid
              (Widget|RemovefromParent _ilde_ui))))))))

(event Input|KeyboardEvents|LeftShift
  (params (Key :type Key%20Structure))
  ;[1 1 1] Zoom Handle
  (:Pressed
    (Variables|Default|Setmodifyer_active true))
  (:Released
    (Variables|Default|Setmodifyer_active false)))

(event Input|MouseEvents|MouseWheelUp
  (params (Key :type Key%20Structure))
  (bind _widget (Variables|Default|GetWidget))
  (bind _min_zoom (Variables|Default|Getmin_zoom))
  ;[1 1 1] Zoom Handle
  (:Pressed
    (Utilities|ModifyerCheck
      (:false
        (Variables|Default|SetSpring%20arm%20length (Math|Float|Clamp(Float) (- (Variables|Default|GetSpring%20arm%20length) 5e+01) _min_zoom 1.3e+03)))
      (:true
        (Variables|Default|SetSpring%20arm%20length (Math|Float|Clamp(Float) (- (Variables|Default|GetSpring%20arm%20length) 2e+02) _min_zoom 1.3e+03))))
    (Variables|/Script/Engine.SpringArmComponent|SetTargetArmLength (Variables|Default|GetSpringArm) (Variables|Default|GetSpring%20arm%20length))
    (Utilities|IsValid _widget
      (:Is%20Valid
        (Default|SetZoomSlider _widget (Math|Float|MapRangeClamped (Variables|Default|GetSpring%20arm%20length) 1.3e+03 (Variables|Default|Getmin_zoom) 0.0 1.0))
        (bind _outactors (Actor|GetAllActorsOfClass "/Game/Blueprints/Turntable/Vehicle_Viewer.Vehicle_Viewer_C"))
        (Utilities|IsValid (Utilities|Array|Get(acopy) _outactors)
          (:Is%20Valid
            (Default|ChangeZoom (Utilities|Array|Get(acopy) _outactors) (Math|Float|MapRangeClamped (Variables|Default|GetSpring%20arm%20length) (Variables|Default|Getmin_zoom) 1.3e+03 0.0 1.0))))))))

(event Input|MouseEvents|RightMouseButton
  (params (Key :type Key%20Structure))
  (bind _returnvalue (Viewport|GetViewportSize))
  (bind _returnvalue_2 (Game|GetPlayerController 0))
  (bind _widget (Variables|Default|GetWidget))
  (:Pressed
    (bind _foundwidgets (Widget|GetAllWidgetsOfClass "/Game/Blueprints/Turntable/User_Interface/TurnTable_Anim_UI.TurnTable_Anim_UI_C" false))
    (Variables|Default|Setanim_widget (Utilities|Array|Get(acopy) _foundwidgets (Utilities|Array|LastIndex _foundwidgets)))
    ;[1 1 1] Hud Toggle
    (if (Variables|Default|Getoverlay_visable)
      (Variables|Default|Setoverlay_visable false)
      (Widget|RemovefromParent _widget)
      (Utilities|IsValid (Variables|Default|Getanim_widget)
        (:Is%20Valid
          (Default|Hide (Variables|Default|Getanim_widget) false))
        (:Is%20Not%20Valid
          _))
      (Variables|/Script/Engine.PlayerController|SetbShowMouseCursor _returnvalue_2 false)
      (Input|SetInputModeGameOnly _returnvalue_2)
      (Class|WidgetBlueprintLibrary|SetFocustoGameViewport)
      (else
        (Variables|Default|Setoverlay_visable true)
        (UserInterface|Viewport|AddtoViewport _widget 0)
        (Utilities|IsValid (Variables|Default|Getanim_widget)
          (:Is%20Valid
            (Default|Hide (Variables|Default|Getanim_widget) true))
          (:Is%20Not%20Valid
            _))
        (Variables|/Script/Engine.PlayerController|SetbShowMouseCursor _returnvalue_2 true)
        (Input|SetInputModeGameandUI _returnvalue_2 0 "DoNotLock" false)
        (Class|PlayerController|SetMouseLocation _returnvalue_2 (/ (Math|Float|Truncate (.x _returnvalue)) 2) (/ (Math|Float|Truncate (.y _returnvalue)) 2))))))

(fn ConstructionScript)