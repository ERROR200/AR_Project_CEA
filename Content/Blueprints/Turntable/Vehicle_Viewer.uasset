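; Turntable showcase actor for a radar vehicle, with auto-rotation, animation playback and cycling material variants.
; Radar isolation swaps the vehicle to an invisible material and radar meshes to translucent ones, shows component groups, and moves Turntable_Pawn between camera points.
; On BeginPlay it links the radar AnimInstance to the animation UI and spawns a Stats actor.
; Zoom lerps five labelled components toward 4x-scaled offsets precomputed in the construction script.
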(event Custom|Kill
  (bind _statsref (Variables|Default|GetStatsRef))
  (Utilities|IsValid _statsref
    (:Is%20Valid
      (Actor|DestroyActor _statsref)
      (Utilities|FlowControl|Delay 0.1))
    (:Is%20Not%20Valid
      _))
  (Actor|DestroyActor))

(event Custom|deploy/stow%20stands
  (params (forward :type Boolean))
  (bind _vehicle_skel_mesh1 (Variables|Default|GetVehicle_Skel_Mesh1))
  (if forward
    (Components|Timeline|SetPlayRate _vehicle_skel_mesh1 1.0)
    (else
      (Components|Timeline|SetPlayRate _vehicle_skel_mesh1 -1.0)))
  (Audio|Components|Audio|Play _vehicle_skel_mesh1 false))

(event Custom|change_zoom
  (params (Alpha :type Float%20%28single-precision%29))
  (for (_array_element _array_index) (Utilities|Array|MakeArray (Variables|Default|GetMEG) (Variables|Default|GetENV) (Variables|Default|GetPWR) (Variables|Default|GetARY) (Variables|Default|GetGEN))
    (Utilities|IsValid _array_element
      (:Is%20Valid
        (Transformation|SetRelativeLocation _array_element (Math|Vector|Lerp(Vector) (Utilities|Array|Get(acopy) (Variables|Default|Getstart%20point%20origins) _array_index) (Variables|/Script/Engine.SceneComponent|GetRelativeLocation (Utilities|Array|Get(acopy) (Utilities|Array|MakeArray (Variables|Default|Getalt_start_point) (Variables|Default|Getalt_start_point2) (Variables|Default|Getalt_start_point3) (Variables|Default|Getalt_start_point4) (Variables|Default|Getalt_start_point5)) _array_index)) Alpha) false false)))))

(event Custom|ForceMatChange
  (params (Index :type Integer))
  (bind _radar_skel_mesh_2 (Variables|Default|GetRadar_Skel_Mesh_2))
  (bind _vehicle (Variables|Default|GetVehicle))
  (bind _secondary_mesh (Variables|Default|GetSecondary_Mesh))
  (bind _radar_skel_mesh_2_2 (Variables|Default|GetRadar_Skel_Mesh_2))
  (bind _radar_skel_mesh (Variables|Default|GetRadar_Skel_Mesh))
  (bind _vehicle_2 (Variables|Default|GetVehicle))
  (bind _secondary_mesh_2 (Variables|Default|GetSecondary_Mesh))
  (Variables|Default|SetMaterial_Index Index)
  (if (> (stale EventSwapTextures _result) (- (Utilities|Array|Length (Variables|Default|GetMaterial_List)) 1))
    (Variables|Default|SetMaterial_Index 0))
  (if (Variables|Default|GetisTransparent)
    (Utilities|IsValid (Utilities|Array|Get(acopy) (Variables|Default|GetRadar_Transl_Material_List) (Variables|Default|GetMaterial_Index))
      (:Is%20Valid
        (Rendering|Material|SetMaterial (Variables|Default|GetRadar_Skel_Mesh) 0 (Utilities|Array|Get(acopy) (Variables|Default|GetRadar_Transl_Material_List) (Variables|Default|GetMaterial_Index))))
      (:Is%20Not%20Valid
        _))
    (Utilities|IsValid _radar_skel_mesh_2_2
      (:Is%20Valid
        (Rendering|Material|SetMaterial _radar_skel_mesh_2_2 0 (Utilities|Array|Get(acopy) (Variables|Default|GetSecondary_Radar_Transl_Material_List) (Variables|Default|GetMaterial_Index))))
      (:Is%20Not%20Valid
        _))
    (Utilities|IsValid _secondary_mesh_2
      (:Is%20Valid
        (Rendering|Material|SetMaterial _secondary_mesh_2 0 (Utilities|Array|Get(acopy) (Variables|Default|GetSecondary_Radar_Transl_Material_List) (Variables|Default|GetMaterial_Index))))
      (:Is%20Not%20Valid
        _))
    (Utilities|IsValid _vehicle_2
      (:Is%20Valid
        (Rendering|Material|SetMaterial _vehicle_2 0 (Variables|Default|GetMaterial_Invisible))))
    (else
      (Rendering|Material|SetMaterial (Variables|Default|GetVehicle_Skel_Mesh1) 0 (Utilities|Array|Get(acopy) (Variables|Default|GetMaterial_List) (Variables|Default|GetMaterial_Index)))
      (Utilities|IsValid _radar_skel_mesh
        (:Is%20Valid
          (Rendering|Material|SetMaterial _radar_skel_mesh 0 (Utilities|Array|Get(acopy) (Variables|Default|GetRadar_Material_List) (Variables|Default|GetMaterial_Index))))
        (:Is%20Not%20Valid
          _))
      (Utilities|IsValid _radar_skel_mesh_2
        (:Is%20Valid
          (Rendering|Material|SetMaterial _radar_skel_mesh_2 0 (Utilities|Array|Get(acopy) (Variables|Default|GetSecondary_Radar_Material_List) (Variables|Default|GetMaterial_Index))))
        (:Is%20Not%20Valid
          _))
      (Utilities|IsValid _secondary_mesh
        (:Is%20Valid
          (Rendering|Material|SetMaterial _secondary_mesh 0 (Utilities|Array|Get(acopy) (Variables|Default|GetSecondary_Radar_Material_List) (Variables|Default|GetMaterial_Index))))
        (:Is%20Not%20Valid
          _))
      (Utilities|IsValid _vehicle
        (:Is%20Valid
          (Rendering|Material|SetMaterial _vehicle 0 (Utilities|Array|Get(acopy) (Variables|Default|GetMaterial_List) (Variables|Default|GetMaterial_Index))))))))

(event EventBeginPlay
  (bind _asturntable_pawn (Utilities|Casting|CastToTurntable_Pawn (Game|Player|GetPlayerPawn 0)))
  (bind _output_get (Variables|Default|Setpawn _asturntable_pawn))
  (CallFunction|ChangeZoom (Math|Float|MapRangeClamped (Variables|/Game/Blueprints/Turntable/Turntable_Pawn.Turntable_Pawn_C|GetSpring%20arm%20length _output_get) 2e+02 1.3e+03 0.0 1.0))
  (Default|HideIdle _output_get)
  (Default|DragScreenMessege _output_get)
  (bind _foundwidgets (Widget|GetAllWidgetsOfClass "/Game/Blueprints/Turntable/User_Interface/TurnTable_Anim_UI.TurnTable_Anim_UI_C" false))
  (Utilities|IsValid (Utilities|Array|Get(acopy) _foundwidgets)
    (:Is%20Valid
      (Variables|Read_Only|Setanim_ui (Utilities|Array|Get(acopy) _foundwidgets)))
    (:Is%20Not%20Valid
      (bind _returnvalue (UserInterface|CreateWidget "/Game/Blueprints/Turntable/User_Interface/TurnTable_Anim_UI.TurnTable_Anim_UI_C"))
      (Variables|Read_Only|Setanim_ui _returnvalue)
      (UserInterface|Viewport|AddtoViewport (Variables|Read_Only|Getanim_ui) 1)))
  (Class|AnimIF|SetupAnim(Message) (Components|SkeletalMesh|GetAnimInstance (Variables|Default|GetRadar_Skel_Mesh)) (Variables|Read_Only|Getanim_ui))
  (Rendering|SetVisibility (Variables|Default|GetRadar_component_group) false true)
  (Variables|Default|SetisTransparent true)
  (CallFunction|IsolateRadar)
  (Utilities|FlowControl|Delay 0.2)
  (bind _returnvalue_2 (Game|SpawnActorfromClass (Variables|Default|GetStats) (Math|Transform|MakeTransform "0, 0, 0" "0, 0, 0" "1,1,1") "Undefined" 0 0))
  (Variables|Default|SetStatsRef _returnvalue_2)
  (Transformation|SetActorLocation (Variables|Default|Getpawn) (Transformation|GetWorldLocation (Variables|Default|GetMain_Cam)) false false))

(event Collision|EventActorBeginOverlap
  (params (OtherActor :type Actor%20Object%20Reference)))

(event EventPlay/PauseAnim
  (bind _anim_ui (Variables|Read_Only|Getanim_ui))
  (bind _radar_skel_mesh (Variables|Default|GetRadar_Skel_Mesh))
  (bind _returnvalue (Components|SkeletalMesh|GetAnimInstance _radar_skel_mesh))
  (Utilities|IsValid _radar_skel_mesh
    (:Is%20Valid
      (if (Variables|Default|GetMulti_mode)
        (Class|AnimIF|SetPlayMode(Message) _returnvalue _anim_ui)
        (else
          (Utilities|FlowControl|FlipFlop
            (:A
              (Class|AnimIF|SetPlayRate(Message) _returnvalue 1.0 _anim_ui))
            (:B
              (Class|AnimIF|SetPlayRate(Message) _returnvalue -1.0 _anim_ui))))))))

(event EventTick
  (params (DeltaSeconds :type Float%20%28single-precision%29))
  (if (Variables|Default|GetisAutoRotate)
    (Transformation|AddLocalRotation (Variables|Default|GetVehicle_Skel_Mesh1) (* "0,1.000000, 0" (* DeltaSeconds (Variables|Default|GetRotateSpeed))) false false)))

(event EventIsolateRadar
  (bind _material_index (Variables|Default|GetMaterial_Index))
  (bind _material_index_2 (Variables|Default|GetMaterial_Index))
  (bind _output_get (Variables|Default|SetisTransparent (not (Variables|Default|GetisTransparent))))
  (if _output_get
    (CallFunction|ToggleIsolation true (Variables|Default|GetMaterial_Invisible) (Utilities|Array|Get(acopy) (Variables|Default|GetRadar_Transl_Material_List) _material_index) (Utilities|Array|Get(acopy) (Variables|Default|GetSecondary_Radar_Transl_Material_List) _material_index) (Transformation|GetWorldLocation (Variables|Default|GetRadar_Cam)))
    (else
      (CallFunction|ToggleIsolation false (Utilities|Array|Get(acopy) (Variables|Default|GetMaterial_List) (Variables|Default|GetMaterial_Index)) (Utilities|Array|Get(acopy) (Variables|Default|GetRadar_Material_List) _material_index_2) (Utilities|Array|Get(acopy) (Variables|Default|GetSecondary_Radar_Material_List) _material_index_2) (Transformation|GetWorldLocation (Variables|Default|GetMain_Cam))))))

(event EventRotate
  (params (Automated :type Boolean) (Speed :type Float%20%28single-precision%29) (Custom_Angle :type Float%20%28single-precision%29))
  (Variables|Default|SetisAutoRotate Automated)
  (Variables|Default|SetRotateSpeed (Math|Float|Clamp(Float) (+ (Variables|Default|GetRotateSpeed) Speed) -3.6e+02 3.6e+02)))

(event EventSwapTextures
  (bind _radar_skel_mesh_2 (Variables|Default|GetRadar_Skel_Mesh_2))
  (bind _vehicle (Variables|Default|GetVehicle))
  (bind _secondary_mesh (Variables|Default|GetSecondary_Mesh))
  (bind _radar_skel_mesh_2_2 (Variables|Default|GetRadar_Skel_Mesh_2))
  (bind _radar_skel_mesh (Variables|Default|GetRadar_Skel_Mesh))
  (bind _vehicle_2 (Variables|Default|GetVehicle))
  (bind _secondary_mesh_2 (Variables|Default|GetSecondary_Mesh))
  (bind _result (Math|Integer|IncrementInt (Variables|Default|GetMaterial_Index))
    (:%20%20
      (if (> _result (- (Utilities|Array|Length (Variables|Default|GetMaterial_List)) 1))
        (Variables|Default|SetMaterial_Index 0))
      (if (Variables|Default|GetisTransparent)
        (Utilities|IsValid (Utilities|Array|Get(acopy) (Variables|Default|GetRadar_Transl_Material_List) (Variables|Default|GetMaterial_Index))
          (:Is%20Valid
            (Rendering|Material|SetMaterial (Variables|Default|GetRadar_Skel_Mesh) 0 (Utilities|Array|Get(acopy) (Variables|Default|GetRadar_Transl_Material_List) (Variables|Default|GetMaterial_Index))))
          (:Is%20Not%20Valid
            _))
        (Utilities|IsValid _radar_skel_mesh_2_2
          (:Is%20Valid
            (Rendering|Material|SetMaterial _radar_skel_mesh_2_2 0 (Utilities|Array|Get(acopy) (Variables|Default|GetSecondary_Radar_Transl_Material_List) (Variables|Default|GetMaterial_Index))))
          (:Is%20Not%20Valid
            _))
        (Utilities|IsValid _secondary_mesh_2
          (:Is%20Valid
            (Rendering|Material|SetMaterial _secondary_mesh_2 0 (Utilities|Array|Get(acopy) (Variables|Default|GetSecondary_Radar_Transl_Material_List) (Variables|Default|GetMaterial_Index))))
          (:Is%20Not%20Valid
            _))
        (Utilities|IsValid _vehicle_2
          (:Is%20Valid
            (Rendering|Material|SetMaterial _vehicle_2 0 (Variables|Default|GetMaterial_Invisible))))
        (else
          (Rendering|Material|SetMaterial (Variables|Default|GetVehicle_Skel_Mesh1) 0 (Utilities|Array|Get(acopy) (Variables|Default|GetMaterial_List) (Variables|Default|GetMaterial_Index)))
          (Utilities|IsValid _radar_skel_mesh
            (:Is%20Valid
              (Rendering|Material|SetMaterial _radar_skel_mesh 0 (Utilities|Array|Get(acopy) (Variables|Default|GetRadar_Material_List) (Variables|Default|GetMaterial_Index))))
            (:Is%20Not%20Valid
              _))
          (Utilities|IsValid _radar_skel_mesh_2
            (:Is%20Valid
              (Rendering|Material|SetMaterial _radar_skel_mesh_2 0 (Utilities|Array|Get(acopy) (Variables|Default|GetSecondary_Radar_Material_List) (Variables|Default|GetMaterial_Index))))
            (:Is%20Not%20Valid
              _))
          (Utilities|IsValid _secondary_mesh
            (:Is%20Valid
              (Rendering|Material|SetMaterial _secondary_mesh 0 (Utilities|Array|Get(acopy) (Variables|Default|GetSecondary_Radar_Material_List) (Variables|Default|GetMaterial_Index))))
            (:Is%20Not%20Valid
              _))
          (Utilities|IsValid _vehicle
            (:Is%20Valid
              (Rendering|Material|SetMaterial _vehicle 0 (Utilities|Array|Get(acopy) (Variables|Default|GetMaterial_List) (Variables|Default|GetMaterial_Index))))))))))

(fn ConstructionScript
  (bind _radar_skel_mesh (Variables|Default|GetRadar_Skel_Mesh))
  (bind _radar_skel_mesh_2 (Variables|Default|GetRadar_Skel_Mesh))
  (bind _env (Variables|Default|GetENV))
  (bind _pwr (Variables|Default|GetPWR))
  (bind _ary (Variables|Default|GetARY))
  (bind _gen (Variables|Default|GetGEN))
  (bind _meg (Variables|Default|GetMEG))
  (bind _relativelocation (Variables|/Script/Engine.SceneComponent|GetRelativeLocation _gen))
  (bind _relativelocation_2 (Variables|/Script/Engine.SceneComponent|GetRelativeLocation _meg))
  (bind _relativelocation_3 (Variables|/Script/Engine.SceneComponent|GetRelativeLocation _env))
  (bind _relativelocation_4 (Variables|/Script/Engine.SceneComponent|GetRelativeLocation _pwr))
  (bind _relativelocation_5 (Variables|/Script/Engine.SceneComponent|GetRelativeLocation _ary))
  (bind _array (Utilities|Array|MakeArray _relativelocation_2 _relativelocation_3 _relativelocation_4 _relativelocation_5 _relativelocation))
  (Utilities|IsValid _radar_skel_mesh
    (:Is%20Valid
      (Transformation|AttachComponentToComponent (Variables|Default|GetRadar_component_group) _radar_skel_mesh (Variables|Default|GetAttach_bone) "KeepRelative" "KeepWorld" "KeepWorld" true))
    (:Is%20Not%20Valid
      _))
  (Utilities|IsValid _radar_skel_mesh_2
    (:Is%20Valid
      (Transformation|AttachComponentToComponent (Variables|Default|GetSecondary_Radar_component_group) _radar_skel_mesh_2 (Variables|Default|GetSecond_Attach_bone) "KeepRelative" "KeepWorld" "KeepWorld" true))
    (:Is%20Not%20Valid
      _))
  (for (_array_element _array_index) _array
    (Transformation|SetRelativeLocation (Utilities|Array|Get(acopy) (Utilities|Array|MakeArray (Variables|Default|Getalt_start_point) (Variables|Default|Getalt_start_point2) (Variables|Default|Getalt_start_point3) (Variables|Default|Getalt_start_point4) (Variables|Default|Getalt_start_point5)) _array_index) (* _array_element 4.0) false false))
  (Variables|Default|Setstart%20point%20origins _array))

(fn ToggleIsolation
  (params (isHidden :type Boolean) (vehicleMat :type Material%20Instance%20Object%20Reference) (radarMat :type Material%20Instance%20Object%20Reference) (secondRadarMat :type Material%20Instance%20Object%20Reference) (cameraLoc :type Vector))
  (bind _pawn (Variables|Default|Getpawn))
  (bind _radar_skel_mesh_2 (Variables|Default|GetRadar_Skel_Mesh_2))
  (bind _secondary_mesh (Variables|Default|GetSecondary_Mesh))
  (bind _radar_skel_mesh (Variables|Default|GetRadar_Skel_Mesh))
  (bind _vehicle (Variables|Default|GetVehicle))
  (Development|SetHiddeninGame (Variables|Default|GetDave) isHidden false)
  (Rendering|Material|SetMaterial (Variables|Default|GetVehicle_Skel_Mesh1) 0 vehicleMat)
  (Utilities|IsValid _radar_skel_mesh
    (:Is%20Valid
      (Rendering|Material|SetMaterial _radar_skel_mesh 0 radarMat))
    (:Is%20Not%20Valid
      _))
  (Transformation|SetActorLocation _pawn cameraLoc false false)
  (Rendering|SetVisibility (Variables|Default|GetTertiary_Radar_component_group) isHidden true)
  (Utilities|IsValid _pawn
    (:Is%20Valid
      (Default|SetZoomLimit _pawn isHidden)
      (Utilities|IsValid _radar_skel_mesh_2
        (:Is%20Valid
          (Rendering|Material|SetMaterial _radar_skel_mesh_2 0 secondRadarMat))
        (:Is%20Not%20Valid
          _))
      (Utilities|IsValid _secondary_mesh
        (:Is%20Valid
          (Rendering|Material|SetMaterial _secondary_mesh 0 secondRadarMat))
        (:Is%20Not%20Valid
          _))
      (Utilities|IsValid _vehicle
        (:Is%20Valid
          (Rendering|Material|SetMaterial _vehicle 0 vehicleMat))
        (:Is%20Not%20Valid
          _))
      (if isHidden
        (Development|ExecuteConsoleCommand "r.PostProcessAAQuality 0" 0)
        (else
          (Development|ExecuteConsoleCommand "r.PostProcessAAQuality 5" 0))))))